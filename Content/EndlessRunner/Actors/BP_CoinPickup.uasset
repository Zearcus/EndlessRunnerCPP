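; BP_CoinPickup is the endless runner's coin pickup, collected when a BP_RunCharacter overlaps its static mesh.
; The overlap fires OnGet, which calls the parent implementation, then adds coins to player 0's character rather than using the overlapping actor.
; It prints the new coin total, plays the coin sound at its location and destroys itself.
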(event OnComponentBeginOverlap(StaticMesh)
  (params (OverlappedComponent :type Primitive%20Component%20Object%20Reference) (OtherActor :type Actor%20Object%20Reference) (OtherComp :type Primitive%20Component%20Object%20Reference) (OtherBodyIndex :type Integer) (bFromSweep :type Boolean) (SweepResult :type Hit%20Result%20Structure%20%28by%20ref%29))
  (Utilities|Casting|CastToBP_RunCharacter OtherActor)
  (Class|RunPickup|OnGet))

(event EventOnGet
  (|CallParentFunction)
  (bind _asbp_run_character (Utilities|Casting|CastToBP_RunCharacter (Game|Player|GetPlayerPawn 0)))
  (Class|RunCharacter|AddCoins _asbp_run_character)
  (Development|PrintString (Utilities|String|ToString(Integer) (Variables|/Script/EndlessRunner.RunCharacter|GetCoins _asbp_run_character)))
  (Audio|PlaySoundatLocation "/Game/EndlessRunner/SFX/coin.coin" (Transformation|GetActorLocation) "0, 0, 0" 1.0 1.0 0.0 0 0 0 0)
  (Actor|DestroyActor))

(fn ConstructionScript)